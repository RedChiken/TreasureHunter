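; Player controller for the lobby that builds the lobby user interface.
; InitializeLobbyUI creates the lobby, group, mission, chat, session browsing and creation, and room member widgets owned by this controller.
; It hands them all to WidgetController.InitializeUI, then switches input to UI only without locking the mouse.
; BeginPlay and Tick are empty, so setup runs only when InitializeLobbyUI is triggered.
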(event EventBeginPlay)

(event EventTick
  (params (DeltaSeconds :type Float%20%28single-precision%29)))

(event EventInitializeLobbyUI
  (bind _self self)
  (Utilities|FlowControl|Sequence
    (:then_0
      (bind _returnvalue (UserInterface|CreateWidget "/Game/UI/Lobby.Lobby_C" _self)))
    (:then_1
      (bind _returnvalue_2 (UserInterface|CreateWidget "/Game/UI/GroupMemberInfo.GroupMemberInfo_C" _self)))
    (:then_2
      (bind _returnvalue_3 (UserInterface|CreateWidget "/Game/UI/MissionInfo.MissionInfo_C" _self)))
    (:then_3
      (bind _returnvalue_4 (UserInterface|CreateWidget "/Game/UI/Chat.Chat_C" _self)))
    (:then_4
      (bind _returnvalue_5 (UserInterface|CreateWidget "/Game/UI/ChatInfo.ChatInfo_C" _self)))
    (:then_5
      (bind _returnvalue_6 (UserInterface|CreateWidget "/Game/UI/FindSession.FindSession_C" _self)))
    (:then_6
      (bind _returnvalue_7 (UserInterface|CreateWidget "/Game/UI/SessionInfo.SessionInfo_C" _self)))
    (:then_7
      (bind _returnvalue_8 (UserInterface|CreateWidget "/Game/UI/CreateSession.CreateSession_C" _self)))
    (:then_8
      (bind _returnvalue_9 (UserInterface|CreateWidget "/Game/UI/Session.Session_C" _self)))
    (:then_9
      (bind _returnvalue_10 (UserInterface|CreateWidget "/Game/UI/RoomMemberInfo.RoomMemberInfo_C" _self)))
    (:then_10
      (Class|WidgetControllerComponent|InitializeUI (Variables|Default|GetWidgetController) _returnvalue _returnvalue_2 _returnvalue_3 _returnvalue_4 _returnvalue_5 _returnvalue_6 _returnvalue_7 _returnvalue_8 _returnvalue_9 _returnvalue_10)
      (Input|SetInputModeUIOnly self 0 "DoNotLock"))))

(fn ConstructionScript)